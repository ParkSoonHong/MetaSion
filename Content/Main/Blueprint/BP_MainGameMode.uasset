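; BP_MainGameMode is a game mode that runs level-specific setup on BeginPlay, based on the current level name.
; In MainRoom it creates the WBP_Controlls widget for the first player controller and adds it to the viewport.
; In MainLobby it spawns a BP_CJS_BallPlayer at SpawnTransform, calls SpawnDefaultController on it, then has the first player controller possess it.
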(event EventBeginPlay
  (bind _returnvalue (Game|GetPlayerController 0))
  (Utilities|FlowControl|Sequence
    (:then_0
      (bind _returnvalue_2 (Game|GetCurrentLevelName true))
      (bind _output_get (Variables|Default|SetLevelname _returnvalue_2))
      (if (Utilities|Enum|Equal(Enum) _output_get (Variables|Default|GetMain_Room))
        (bind _returnvalue_3 (UserInterface|CreateWidget "/Game/KGw/UI/WBP_Controlls.WBP_Controlls_C" (Game|GetPlayerController 0)))
        (UserInterface|Viewport|AddtoViewport _returnvalue_3 0)))
    (:then_1
      (bind _returnvalue_4 (Game|GetCurrentLevelName true))
      (bind _output_get_2 (Variables|Default|SetLevelname _returnvalue_4))
      (if (Utilities|Enum|Equal(Enum) _output_get_2 (Variables|Default|GetMain_Lobby))
        (bind _returnvalue_5 (Game|SpawnActorfromClass "/Game/CJS/Blueprints/BP_CJS_BallPlayer.BP_CJS_BallPlayer_C" (Variables|Default|GetSpawnTransform) "Undefined" "MultiplyWithRoot" _returnvalue 0))
        (Pawn|SpawnDefaultController _returnvalue_5)
        (Pawn|Possess _returnvalue _returnvalue_5)))))

(event EventTick
  (params (DeltaSeconds :type Float%20%28single-precision%29)))

(fn ConstructionScript)