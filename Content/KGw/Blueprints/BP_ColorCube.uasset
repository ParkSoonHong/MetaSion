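; BP_ColorCube is a cube actor set up for recoloring through a UI widget.
; BeginPlay enables player input and adds a hidden WBP_Controller to the viewport.
; NewFunction creates a dynamic M_CubeColor material instance, but nothing here calls it.
; Disconnected logic would toggle the widget and cursor, and map a slider to hue via HSV-to-RGB for an unnamed material parameter.
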(event EventBeginPlay
  (Input|EnableInput (Game|GetPlayerController 0))
  (bind _returnvalue (UserInterface|CreateWidget "/Game/KGw/UI/WBP_Controller.WBP_Controller_C"))
  (bind _output_get (Variables|Default|Setwidget _returnvalue))
  (UserInterface|Viewport|AddtoViewport _output_get 0)
  (Widget|SetVisibility _output_get "Hidden"))

(event Collision|EventActorBeginOverlap
  (params (OtherActor :type Actor%20Object%20Reference)))

(event EventTick
  (params (DeltaSeconds :type Float%20%28single-precision%29)))

(event Input|KeyboardEvents|0
  (params (Key :type Key%20Structure)))

(fn ConstructionScript)

(fn NewFunction
  (bind _returnvalue (Rendering|Material|CreateDynamicMaterialInstance (Variables|Default|GetCube) 0 "/Game/KGw/MAterial/M_CubeColor.M_CubeColor" "None" :!class /Script/Engine.PrimitiveComponent))
  (Variables|Default|SetDYnamicMaterial _returnvalue))