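; Player controller for a rolling-ball player, caching the possessed BP_Jk_Player on BeginPlay.
; Each tick it polls WASD and pushes the Ball component with mass-independent forces along the camera's forward and right vectors.
; Mouse axes drive yaw and inverted-sign pitch input.
; Space applies an upward velocity-change impulse gated by CanJump, which is cleared on use and never reset within this graph.
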(event EventBeginPlay
  (bind _asbp_jk_player (Utilities|Casting|CastToBP_Jk_Player (Pawn|GetControlledPawn)))
  (Variables|Default|SetBP%20Jk%20Player _asbp_jk_player))

(event EventTick
  (params (DeltaSeconds :type Float%20%28single-precision%29))
  (bind _bp_jk_player (Variables|Default|GetBP%20Jk%20Player))
  (bind _bp_jk_player_2 (Variables|Default|GetBP%20Jk%20Player))
  (bind _bp_jk_player_3 (Variables|Default|GetBP%20Jk%20Player))
  (bind _bp_jk_player_4 (Variables|Default|GetBP%20Jk%20Player))
  (Utilities|FlowControl|Sequence
    (:then_0
      ;[1 1 1] W Key
      (if (Game|Player|IsInputKeyDown "W")
        (Physics|AddForce (Variables|/Game/Junguk/Player_ball/BP_Jk_Player.BP_Jk_Player_C|GetBall _bp_jk_player_2) (* (Math|Vector|GetForwardVector (Variables|/Game/Junguk/Player_ball/BP_Jk_Player.BP_Jk_Player_C|GetCamera _bp_jk_player_2)) 1e+03) "None" true)))
    (:then_1
      ;[1 1 1] S Key
      (if (Game|Player|IsInputKeyDown "S")
        (Physics|AddForce (Variables|/Game/Junguk/Player_ball/BP_Jk_Player.BP_Jk_Player_C|GetBall _bp_jk_player_3) (* (Math|Vector|GetForwardVector (Variables|/Game/Junguk/Player_ball/BP_Jk_Player.BP_Jk_Player_C|GetCamera _bp_jk_player_3)) -1e+03) "None" true)))
    (:then_2
      ;[1 1 1] A Key
      (if (Game|Player|IsInputKeyDown "A")
        (Physics|AddForce (Variables|/Game/Junguk/Player_ball/BP_Jk_Player.BP_Jk_Player_C|GetBall _bp_jk_player_4) (* (Math|Vector|GetRightVector (Variables|/Game/Junguk/Player_ball/BP_Jk_Player.BP_Jk_Player_C|GetCamera _bp_jk_player_4)) -1e+03) "None" true)))
    (:then_3
      ;[1 1 1] D Key
      (if (Game|Player|IsInputKeyDown "D")
        (Physics|AddForce (Variables|/Game/Junguk/Player_ball/BP_Jk_Player.BP_Jk_Player_C|GetBall _bp_jk_player) (* (Math|Vector|GetRightVector (Variables|/Game/Junguk/Player_ball/BP_Jk_Player.BP_Jk_Player_C|GetCamera _bp_jk_player)) 1e+03) "None" true)))))

(event Input|MouseEvents|MouseX
  (params (AxisValue :type Float%20%28single-precision%29))
  (Class|PlayerController|AddYawInput AxisValue))

(event Input|MouseEvents|MouseY
  (params (AxisValue :type Float%20%28single-precision%29))
  (Class|PlayerController|AddPitchInput (* AxisValue -1.0)))

(event Input|KeyboardEvents|SpaceBar
  (params (Key :type Key%20Structure :default "None"))
  (:Pressed
    (if (Variables|Default|GetCan_Jump)
      (Variables|Default|SetCan_Jump false)
      (Physics|AddImpulse (Variables|/Game/Junguk/Player_ball/BP_Jk_Player.BP_Jk_Player_C|GetBall (Variables|Default|GetBP%20Jk%20Player)) "0.000000,0.000000,1000.000000" "None" true))))

(fn ConstructionScript)