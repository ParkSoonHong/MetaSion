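; BP_RenderTarget_PaintingCanvers is a mouse-painted canvas actor that draws into a render target, which it clears on BeginPlay.
; Each Tick it line-traces its static mesh using the hit location under the cursor.
; While left mouse is held on a hit, FindCollisionUV converts the hit to render target coordinates, where Canvas DrawPolygon stamps a small round brush dot.
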(event EventBeginPlay
  (bind _paintingrendertarget (Variables|Default|GetPaintingRenderTarget))
  ;[1 1 1] clear UVTarget
  (Rendering|ClearRenderTarget2D _paintingrendertarget (Variables|/Script/Engine.TextureRenderTarget2D|GetClearColor _paintingrendertarget)))

(event Collision|EventActorBeginOverlap
  (params (OtherActor :type Actor%20Object%20Reference)))

(event EventTick
  (params (DeltaSeconds :type Float%20%28single-precision%29))
  (bind _returnvalue (Game|GetPlayerController 0))
  (bind _hitresult (Game|Player|GetHitResultUnderCursorbyChannel _returnvalue "TraceTypeQuery1" true))
  (bind _location (Collision|BreakHitResult _hitresult))
  ;[1 1 1] Painting Actor
  (bind (_hitlocation _hitnormal _bonename _outhit _returnvalue_2) (Collision|LineTraceComponent (Variables|Default|GetStaticMesh) _location (* _location 1e+04) true false false))
  (if _returnvalue_2
    (if (Game|Player|IsInputKeyDown _returnvalue "LeftMouseButton")
      (bind (_canvas _size) (Rendering|BeginDrawCanvastoRenderTarget (Variables|Default|GetPaintingRenderTarget)))
      (Class|Canvas|DrawPolygon _canvas 0 (* _size (.UV (Class|GameplayStatics|FindCollisionUV _outhit))) "(X=10.000000,Y=10.000000)" 16 "(R=1.000000,G=1.000000,B=1.000000,A=1.000000)"))))

(fn ConstructionScript)